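; Test player pawn with Enhanced Input movement, look controls, an attack and an orbiting shield ability.
; Attack spawns a BP_TestActor just ahead of the pawn, while look input yaws the controller and pitches the spring arm.
; Shield spawns a BP_TestShield attached to the Rotation component spun by RotatingMovement; only the first loop index is wired.
; Tick runs the cooldown that re-enables the shield.
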(event `EnhancedInput|/Game/Test/TestInput/IA_TestShield`
  (params (ActionValue :type Boolean) (ElapsedSeconds :type "Float (double-precision)") (TriggeredSeconds :type "Float (double-precision)") (InputAction :type "InputAction Object Reference" :default "/Game/Test/TestInput/IA_TestShield.IA_TestShield"))
  (:`Started`
    (if (`self.ShieldEnable`)
      (set `self.ShieldEnable` false)
      (for _index (range 4)
        (switch `int` _index
          (:`0`
            (bind _returnvalue (`|SpawnActorFromClass` "/Game/Test/TestBlueprint/BP_TestShield.BP_TestShield_C" (`KismetMathLibrary.MakeTransform` (* (`self.GetActorForwardVector`) 200.0)) "Undefined" "MultiplyWithRoot" null null))
            (`self.K2_AttachToComponent` _returnvalue (`self.Rotation`) "None" "KeepRelative" "KeepRelative" "KeepRelative" true)))))))

(event `EnhancedInput|/Game/Test/TestInput/IA_TestAttack`
  (params (ActionValue :type Boolean) (ElapsedSeconds :type "Float (double-precision)") (TriggeredSeconds :type "Float (double-precision)") (InputAction :type "InputAction Object Reference" :default "/Game/Test/TestInput/IA_TestAttack.IA_TestAttack"))
  (:`Started`
    (`|SpawnActorFromClass` "/Game/Test/TestBlueprint/BP_TestActor.BP_TestActor_C" (`KismetMathLibrary.MakeTransform` (+ (`self.K2_GetActorLocation`) (* (`self.GetActorForwardVector`) 100.0)) (`self.K2_GetActorRotation`)) "Undefined" "MultiplyWithRoot" null null)))

(event `EnhancedInput|/Game/Test/TestInput/IA_TestMove`
  (params (ActionValue :type "Vector2D Structure") (ElapsedSeconds :type "Float (double-precision)") (TriggeredSeconds :type "Float (double-precision)") (InputAction :type "InputAction Object Reference" :default "/Game/Test/TestInput/IA_TestMove.IA_TestMove"))
  (bind (_x _y) (`KismetMathLibrary.BreakVector2D` ActionValue))
  (:`Triggered`
    (`|ExecutionSequence`
      (:`then_0`
        (`self.AddMovementInput` (`self.GetActorRightVector`) _x))
      (:`then_1`
        (`self.AddMovementInput` (`self.GetActorForwardVector`) _y)))))

(event `self.ReceiveBeginPlay`
  (message `EnhancedInputSubsystemInterface.AddMappingContext` (pcsubsystem `EnhancedInputLocalPlayerSubsystem` (`GameplayStatics.GetPlayerController` 0)) "/Game/Test/TestInput/IMC_Test.IMC_Test" 0 (struct))
  (`MovementComponent.SetUpdatedComponent` (`self.RotatingMovement`) (`self.Rotation`)))

(event `self.ReceiveTick`
  (params (DeltaSeconds :type "Float (single-precision)"))
  (if (not (`self.ShieldEnable`))
    (bind _output_get (set `self.ShieldTime` (+ DeltaSeconds (`self.ShieldTime`))))
    (if (>= _output_get 6.0)
      (set `self.ShieldEnable` true)
      (set `self.ShieldTime` 0.0))))

(event `EnhancedInput|/Game/Test/TestInput/IA_TestRotation`
  (params (ActionValue :type "Vector2D Structure") (ElapsedSeconds :type "Float (double-precision)") (TriggeredSeconds :type "Float (double-precision)") (InputAction :type "InputAction Object Reference" :default "/Game/Test/TestInput/IA_TestRotation.IA_TestRotation"))
  (bind (_x _y) (`KismetMathLibrary.BreakVector2D` ActionValue))
  (:`Triggered`
    (`self.AddControllerYawInput` _x)
    (`SceneComponent.K2_AddRelativeRotation` (`self.SpringArm`) (`KismetMathLibrary.MakeRotator` 0.0 (* _y 90.0 (`GameplayStatics.GetWorldDeltaSeconds`))) false false)))

(fn `UserConstructionScript`)